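; BP_PTLHUD is a HUD Blueprint with logic to draw a target-lock indicator over the player's locked enemy.
; That logic is disconnected from DrawHUD, so the HUD currently draws nothing.
; The unused chain gets the enemy from the PTLPlayer's target lock component, projects its target component's location to screen space and centres the indicator texture there.
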(event `self.ReceiveDrawHUD`
  (params (SizeX :type Integer) (SizeY :type Integer)))

(fn `UserConstructionScript`)